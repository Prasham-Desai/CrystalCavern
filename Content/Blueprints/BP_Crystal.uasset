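; BP_Crystal is a crystal actor that flies to the player on overlap and then destroys itself.
; An overlap with the player pawn plays the CrystalPositionLerp timeline, whose alpha track feeds MoveCrystalToPlayer on every update.
; That function lerps from the crystal's current location, not a stored start, toward the pawn's live position, so it homes on a moving player.
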(event `self.ReceiveActorBeginOverlap`
  (params (OtherActor :type "Actor Object Reference"))
  ;[0.05156 0 0.15 0.5] Crystal Collision
  (if (== OtherActor (`GameplayStatics.GetPlayerPawn` 0))
    (bind (_direction _crystal_position) (`Timeline|Crystal Position Lerp`)
      (:`Update`
        (`self.MoveCrystalToPlayer` _crystal_position))
      (:`Finished`
        (`self.K2_DestroyActor`)))))

(fn `MoveCrystalToPlayer`
  (params (Alpha :type "Float (single-precision)"))
  ;[0.15 0.01739 0.0911 0.5] Moving Crystal To Player
  (`self.K2_SetActorLocation` (`KismetMathLibrary.VLerp` (`self.K2_GetActorLocation`) (`self.K2_GetActorLocation` (`GameplayStatics.GetPlayerPawn` 0)) Alpha)))

(fn `UserConstructionScript`)