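; Demo player pawn driven with tank-style differential steering through Enhanced Input, with the input mapping context added on BeginPlay.
; Forward/backward and turn actions share one path that sums and subtracts action values into clamped left and right wheel forces.
; Each force, scaled by a multiplier, pushes the physics mesh along local X at its wheel set's location.
; Completing either action zeroes both stored forces.
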(event `self.ReceiveBeginPlay`
  (`EnhancedInputSubsystemInterface.AddMappingContext` (pcsubsystem `EnhancedInputLocalPlayerSubsystem` (`GameplayStatics.GetPlayerController` 0)) "/Game/InputMapping.InputMapping" 0 (struct)))

(event `EnhancedInput|/Game/IA_ForwardsBackwards`
  (params (ActionValue :type "Float (double-precision)") (ElapsedSeconds :type "Float (double-precision)") (TriggeredSeconds :type "Float (double-precision)") (InputAction :type "InputAction Object Reference" :default "/Game/IA_ForwardsBackwards.IA_ForwardsBackwards"))
  (:`Triggered`
    (set `self.LeftWheelForce` (`KismetMathLibrary.FClamp` (+ ActionValue (stale `EnhancedInput|/Game/IA_Turn` ActionValue)) -1.0) :!label _label)
    (set `self.RightWheelForce` (`KismetMathLibrary.FClamp` (- ActionValue (stale `EnhancedInput|/Game/IA_Turn` ActionValue)) -1.0))
    (`PrimitiveComponent.AddForceAtLocationLocal` (`self.PlayerMesh`) (`KismetMathLibrary.MakeVector` (* (`self.LeftWheelForce`) (`self.ForceMultiplier`))) (`SceneComponent.RelativeLocation` (`self.LeftWheels`)) "None") ; Left Wheel Force
    (`PrimitiveComponent.AddForceAtLocationLocal` (`self.PlayerMesh`) (`KismetMathLibrary.MakeVector` (* (`self.RightWheelForce`) (`self.ForceMultiplier`))) (`SceneComponent.RelativeLocation` (`self.RightWheels`)) "None") ; Right Wheel Force
  )
  (:`Completed`
    (set `self.LeftWheelForce` 0.0 :!label _label_2)
    (set `self.RightWheelForce` 0.0)))

(event `EnhancedInput|/Game/IA_Turn`
  (params (ActionValue :type "Float (double-precision)") (ElapsedSeconds :type "Float (double-precision)") (TriggeredSeconds :type "Float (double-precision)") (InputAction :type "InputAction Object Reference" :default "/Game/IA_Turn.IA_Turn"))
  (:`Triggered`
    (goto _label))
  (:`Completed`
    (goto _label_2)))

(fn `UserConstructionScript`)