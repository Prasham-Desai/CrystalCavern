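; BP_Cannon is an automatic cannon that repeatedly fires BP_Projectile actors, starting at BeginPlay.
; After each shoot-rate delay, it spawns a projectile at the Arrow component's world transform, scaled by CannonBallScale.
; The CannonAnim timeline then animates the Cannon component along its relative Y axis.
; The timeline's Cannon Fire Start event track loops execution back to the delay for the next shot.
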(event `self.ReceiveBeginPlay`
  (`KismetSystemLibrary.Delay` (`self.CannonShootRate`) :!label _label)
  (`self.Spawn Projectile`)
  (bind (_direction _newtrack_0) (`Timeline|CannonAnim` :`NewTime` 0.5 :!via `PlayFromStart`)
    (:`Update`
      (`self.MoveCannon` _newtrack_0))
    (:`CannonFireStart`
      (goto _label))))

(fn `MoveCannon`
  (params (CannonLocation :type "Float (double-precision)"))
  (`SceneComponent.K2_SetRelativeLocation` (`self.Cannon`) (`KismetMathLibrary.MakeVector` 0.0 CannonLocation) false false))

(fn `Spawn Projectile`
  (bind _arrow (`self.Arrow`))
  (`|SpawnActorFromClass` "/Game/Blueprints/BP_Projectile.BP_Projectile_C" (`KismetMathLibrary.MakeTransform` (`SceneComponent.K2_GetComponentLocation` _arrow) (`SceneComponent.K2_GetComponentRotation` _arrow) (`KismetMathLibrary.Conv_DoubleToVector` (`self.CannonBallScale`))) "Undefined" "MultiplyWithRoot" null null))

(fn `UserConstructionScript`)