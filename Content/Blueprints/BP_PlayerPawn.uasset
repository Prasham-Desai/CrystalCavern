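; Player pawn for a physics-driven drill vehicle that uses Enhanced Input and tank-style differential steering.
; Vertical and horizontal input are mixed into clamped left and right wheel forces, applied to the mesh at each wheel set's location.
; Input start and completion events drive fades for forward and turning audio.
; Taking damage once fades the camera and reloads the level; a helper sets spring arm length and pitch.
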(event `self.ReceiveBeginPlay`
  ;[0.15 0 0.1125 0.5] Adding Input Mapping Context
  (`EnhancedInputSubsystemInterface.AddMappingContext` (pcsubsystem `EnhancedInputLocalPlayerSubsystem` (`GameplayStatics.GetPlayerController` 0)) "/Game/InputActions/IMC_DrillMovement.IMC_DrillMovement" 0 (struct)))

(event `EnhancedInput|/Game/InputActions/IA_Vertical`
  (params (ActionValue :type "Float (double-precision)") (ElapsedSeconds :type "Float (double-precision)") (TriggeredSeconds :type "Float (double-precision)") (InputAction :type "InputAction Object Reference" :default "/Game/InputActions/IA_Vertical.IA_Vertical"))
  ;[0.15 0.09553 0 0.5] Tank Differential Movement
  (:`Triggered`
    (`self.ApplyWheelForce` ActionValue ActionValue (stale `EnhancedInput|/Game/InputActions/IA_Horizontal` ActionValue) (stale `EnhancedInput|/Game/InputActions/IA_Horizontal` ActionValue) :!label _label))
  (:`Started`
    (`self.Movement Audio` :!label _label_2)
    (`self.SetWheelForceToZeroOnCompletion`)
    (goto _label_2 :!via `execute2`))
  (:`Completed`
    (goto _label_2 :!via `execute2`)))

(event `EnhancedInput|/Game/InputActions/IA_Horizontal`
  (params (ActionValue :type "Float (double-precision)") (ElapsedSeconds :type "Float (double-precision)") (TriggeredSeconds :type "Float (double-precision)") (InputAction :type "InputAction Object Reference" :default "/Game/InputActions/IA_Horizontal.IA_Horizontal"))
  ;[0.15 0.09553 0 0.5] Tank Differential Movement
  (:`Triggered`
    (goto _label))
  (:`Started`
    (goto _label_2 :!via `execute3`))
  (:`Completed`
    (goto _label_2 :!via `execute4`)))

(event `self.ReceiveAnyDamage`
  (params (Damage :type "Float (single-precision)") (DamageType :type "DamageType Object Reference") (InstigatedBy :type "Controller Object Reference") (DamageCauser :type "Actor Object Reference"))
  ;[0.15 0 0.009439 0.5] On Player Damaged
  (`/Engine/EditorBlueprintResources/StandardMacros.DoOnce` false
    (:`Completed`
      (`self.RestartLevel`))))

(fn `AdjustSpringArm`
  (params (CamDist :type "Float (double-precision)" :default 500.0) (CamPitch :type "Float (double-precision)" :default -39.0))
  (bind _springarm (`self.SpringArm`))
  (set `SpringArmComponent.TargetArmLength` CamDist _springarm)
  (`SceneComponent.K2_SetWorldRotation` _springarm (`KismetMathLibrary.MakeRotator` 0.0 CamPitch) false false))

(fn `ApplyForceToLeftWheel`
  (`PrimitiveComponent.AddForceAtLocationLocal` (`self.PlayerMesh`) (`KismetMathLibrary.MakeVector` (* (`self.LeftWheelForce`) (`self.ForceMultiplier`))) (`SceneComponent.RelativeLocation` (`self.LeftWheels`)) "None") ; Left Wheel Force
)

(fn `ApplyForceToRightWheel`
  (`PrimitiveComponent.AddForceAtLocationLocal` (`self.PlayerMesh`) (`KismetMathLibrary.MakeVector` (* (`self.RightWheelForce`) (`self.ForceMultiplier`))) (`SceneComponent.RelativeLocation` (`self.RightWheels`)) "None") ; Right Wheel Force
)

(fn `ApplyWheelForce`
  (params (A2 :type "Float (double-precision)") (A :type "Float (double-precision)") (B2 :type "Float (double-precision)") (B :type "Float (double-precision)"))
  (`self.GetActionValueAndClamp` A A2 B B2)
  (`self.ApplyForceToLeftWheel`)
  (`self.ApplyForceToRightWheel`))

(fn `GetActionValueAndClamp`
  (params (A :type "Float (double-precision)") (A2 :type "Float (double-precision)") (B :type "Float (double-precision)") (B2 :type "Float (double-precision)"))
  (set `self.LeftWheelForce` (`KismetMathLibrary.FClamp` (+ A2 B2) -1.0))
  (set `self.RightWheelForce` (`KismetMathLibrary.FClamp` (- A B) -1.0)))

(fn `SetWheelForceToZeroOnCompletion`
  (set `self.LeftWheelForce` 0.0)
  (set `self.RightWheelForce` 0.0))

(fn `UserConstructionScript`)